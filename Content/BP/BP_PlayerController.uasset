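; BP_PlayerController is a player controller that routes movement, look, jump and fire input to player character 0.
; Move axes use the controller's own forward and right vectors, while Turn and LookUp add yaw and pitch input.
; Fire casts the character to BP_Player and calls Firing, then runs a debug-drawn visibility trace from the controller's location to a fixed world point, leaving the result unused.
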(event Input|ActionEvents|InputActionJump
  (params (Key :type Key%20Structure :default "None"))
  (:Pressed
    (Character|Jump (Game|GetPlayerCharacter 0))))

(event Input|ActionEvents|InputActionFire
  (params (Key :type Key%20Structure :default "None"))
  (:Pressed
    (bind _asbp_player (Utilities|Casting|CastToBP_Player (Game|GetPlayerCharacter 0)))
    (Default|Firing _asbp_player)
    (Collision|LineTraceByChannel (Transformation|GetActorLocation (Game|GetPlayerController 0)) "1000.000000, 0, 0" "TraceTypeQuery1" false 0 "ForDuration" true "(R=1.000000,G=0.000000,B=0.000000,A=1.000000)" "(R=0.000000,G=1.000000,B=0.000000,A=1.000000)" 3.0)))

(event Input|AxisEvents|InputAxisMoveForward
  (params (AxisValue :type Float%20%28single-precision%29))
  (Pawn|Input|AddMovementInput (Game|GetPlayerCharacter 0) (Transformation|GetActorForwardVector) AxisValue false))

(event Input|AxisEvents|InputAxisMoveRight
  (params (AxisValue :type Float%20%28single-precision%29))
  (Pawn|Input|AddMovementInput (Game|GetPlayerCharacter 0) (Transformation|GetActorRightVector) AxisValue false))

(event Input|AxisEvents|InputAxisTurn
  (params (AxisValue :type Float%20%28single-precision%29))
  (Pawn|Input|AddControllerYawInput (Game|GetPlayerCharacter 0) AxisValue))

(event Input|AxisEvents|InputAxisLookUp
  (params (AxisValue :type Float%20%28single-precision%29))
  (Pawn|Input|AddControllerPitchInput (Game|GetPlayerCharacter 0) AxisValue))

(fn ConstructionScript)