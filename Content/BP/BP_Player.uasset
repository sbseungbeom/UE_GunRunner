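; BP_Player is the player Blueprint, tracking score, health and a firing animation.
; Capsule overlaps with actors tagged "UnOverlapped" add a point, guarded by a flag that clears on end overlap, which also raises AddScore.
; Hitting BP_Obstacle calls Damaged to lower HP and flag DecreaseHp, then a delay-gated flag blocks further damage briefly.
; Firing plays the player montage, and BeginPlay sets MaxHP.
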(event OnComponentBeginOverlap(CapsuleComponent)
  (params (OverlappedComponent :type Primitive%20Component%20Object%20Reference) (OtherActor :type Actor%20Object%20Reference) (OtherComp :type Primitive%20Component%20Object%20Reference) (OtherBodyIndex :type Integer) (bFromSweep :type Boolean) (SweepResult :type Hit%20Result%20Structure%20%28by%20ref%29))
  ;[1 1 1] 점수 제어
  (if (not (Variables|Default|Getb_IsOverlapped))
    (if (Actor|ActorHasTag OtherActor "UnOverlapped")
      (Variables|Default|SetScore (+ (Variables|Default|GetScore) 1))
      (Variables|Default|Setb_IsOverlapped true))))

(event OnComponentEndOverlap(CapsuleComponent)
  (params (OverlappedComponent :type Primitive%20Component%20Object%20Reference) (OtherActor :type Actor%20Object%20Reference) (OtherComp :type Primitive%20Component%20Object%20Reference) (OtherBodyIndex :type Integer))
  ;[1 1 1] 점수 제어
  (Variables|Default|Setb_IsOverlapped false)
  (Variables|Default|SetbAddScore true))

(event OnComponentHit(CapsuleComponent)
  (params (HitComponent :type Primitive%20Component%20Object%20Reference) (OtherActor :type Actor%20Object%20Reference) (OtherComp :type Primitive%20Component%20Object%20Reference) (NormalImpulse :type Vector :default "0, 0, 0") (Hit :type Hit%20Result%20Structure%20%28by%20ref%29))
  ;[1 1 1] 장애물과 충돌 시 / DAMAGED 함수 실행,3초간 무적(딜레이)
  (if (== (Utilities|GetClass OtherActor) "/Game/BP/BP_Obstacle.BP_Obstacle_C")
    (if (not (Variables|Default|Getb_isCollidedWithObstacle))
      (Variables|Default|Setb_isCollidedWithObstacle true)
      (CallFunction|Damaged)
      (Utilities|FlowControl|Delay 3.0)
      (Variables|Default|Setb_isCollidedWithObstacle false))))

(event EventBeginPlay
  (Variables|Default|SetMaxHP 5))

(fn ConstructionScript)

(fn Damaged
  (if (>= (Variables|Default|GetHP) 1)
    (Variables|Default|SetbDecreaseHp true)
    (bind _result (Math|Integer|DecrementInt (Variables|Default|GetHP))
      (:%20%20
        (Variables|Default|SetHP _result)))))

(fn Firing
  (Animation|PlayAnimMontage "/Game/Animations/AM_Player.AM_Player" 1.0 "None"))