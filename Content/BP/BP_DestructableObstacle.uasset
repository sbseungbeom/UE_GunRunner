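; BP_DestructableObstacle is an obstacle actor that moves when its box is overlapped and tracks a destructible state.
; Box begin overlap plays a timeline that drives the actor's relative location, and end overlap reverses it after a short delay.
; BeginPlay initializes ObstacleHP, and Tick polls it to set the Destruct flag at zero.
; Nothing in these graphs reduces the HP or acts on that flag.
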(event OnComponentBeginOverlap(Box)
  (params (OverlappedComponent :type Primitive%20Component%20Object%20Reference) (OtherActor :type Actor%20Object%20Reference) (OtherComp :type Primitive%20Component%20Object%20Reference) (OtherBodyIndex :type Integer) (bFromSweep :type Boolean) (SweepResult :type Hit%20Result%20Structure%20%28by%20ref%29))
  (bind _새_트랙_0 (Timeline|타임라인_0 Play)
    (:Update
      (Transformation|SetActorRelativeLocation _새_트랙_0))))

(event OnComponentEndOverlap(Box)
  (params (OverlappedComponent :type Primitive%20Component%20Object%20Reference) (OtherActor :type Actor%20Object%20Reference) (OtherComp :type Primitive%20Component%20Object%20Reference) (OtherBodyIndex :type Integer))
  (Utilities|FlowControl|Delay 2.0)
  (bind _새_트랙_0 (Timeline|타임라인_0 Reverse)
    (:Update
      (Transformation|SetActorRelativeLocation _새_트랙_0))))

(event EventBeginPlay
  (Variables|Default|SetObstacleHP 5)
  (Variables|Default|SetbDestruct false))

(event Collision|EventActorBeginOverlap
  (params (OtherActor :type Actor%20Object%20Reference)))

(event EventTick
  (params (DeltaSeconds :type Float%20%28single-precision%29))
  (if (== (Variables|Default|GetObstacleHP) 0)
    (Variables|Default|SetbDestruct true)))

(fn ConstructionScript)