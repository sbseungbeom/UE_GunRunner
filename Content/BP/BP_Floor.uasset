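; BP_Floor is a self-extending track segment for an endless-runner style level.
; When BP_Player first overlaps its Box, a bool guard lets it spawn the next BP_Floor ahead along X and a BP_Obstacle in one of three random Y lanes.
; Its tag starts as UnOverlapped and becomes Overlapped on any Box end overlap, intended to prevent scoring twice on the same floor.
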(event OnComponentEndOverlap(Box)
  (params (OverlappedComponent :type Primitive%20Component%20Object%20Reference) (OtherActor :type Actor%20Object%20Reference) (OtherComp :type Primitive%20Component%20Object%20Reference) (OtherBodyIndex :type Integer))
  ;[1 1 1] 장애물, 지형 생성 / 이미 점수를 얻은 FLoor에서 점수를 얻지 못하도록 set tag
  (Variables|Default|SetTags (Utilities|Array|MakeArray "Overlapped")))

(event OnComponentBeginOverlap(Box)
  (params (OverlappedComponent :type Primitive%20Component%20Object%20Reference) (OtherActor :type Actor%20Object%20Reference) (OtherComp :type Primitive%20Component%20Object%20Reference) (OtherBodyIndex :type Integer) (bFromSweep :type Boolean) (SweepResult :type Hit%20Result%20Structure%20%28by%20ref%29))
  (bind _returnvalue (Transformation|GetActorLocation))
  (bind _returnvalue_2 (Actor|GetActorOfClass "/Game/BP/BP_Player.BP_Player_C"))
  ;[1 1 1] 장애물, 지형 생성 / 이미 점수를 얻은 FLoor에서 점수를 얻지 못하도록 set tag
  (if (== _returnvalue_2 OtherActor)
    (if (not (Variables|Default|Getb_isOverlapped))
      (Variables|Default|Setb_isOverlapped true)
      (Game|SpawnActorfromClass "BP_Floor_C" (Math|Conversions|ToTransform(Vector) (+ (Transformation|GetActorLocation) "2000.000000,0,0")) "Undefined" 0 0)
      (switch int (Math|Conversions|ToInteger(Byte) (Class|KismetMathLibrary|RandomInteger64inRange 0 2))
        (:0
          (Game|SpawnActorfromClass "/Game/BP/BP_Obstacle.BP_Obstacle_C" (Math|Conversions|ToTransform(Vector) (+ _returnvalue "1900.000000,-200.000000,0.000000")) "Undefined" 0 0))
        (:1
          (Game|SpawnActorfromClass "/Game/BP/BP_Obstacle.BP_Obstacle_C" (Math|Conversions|ToTransform(Vector) (+ _returnvalue "1900.000000,0.000000,0.000000")) "Undefined" 0 0))
        (:2
          (Game|SpawnActorfromClass "/Game/BP/BP_Obstacle.BP_Obstacle_C" (Math|Conversions|ToTransform(Vector) (+ _returnvalue "1900.000000,200.000000,0.000000")) "Undefined" 0 0))))))

(event EventBeginPlay
  ;[1 1 1] 장애물, 지형 생성 / 이미 점수를 얻은 FLoor에서 점수를 얻지 못하도록 set tag
  (Variables|Default|SetTags (Utilities|Array|MakeArray "UnOverlapped")))

(event Collision|EventActorBeginOverlap
  (params (OtherActor :type Actor%20Object%20Reference)))

(event EventTick
  (params (DeltaSeconds :type Float%20%28single-precision%29)))

(fn ConstructionScript)